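; BP_Torretta is a turret actor that tracks and shoots at the player within a trigger distance.
; Tick checks the distance to the player pawn and yaws the Cylinder toward it while in range.
; A looping timer fires a debug-drawn line trace from ShootingDirection, sends a damage interface message to the hit actor and restarts the muzzle flash.
; Each shot also plays a Timeline that slides the Cannon along its local X axis.
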(event `self.ReceiveTick`
  (params (DeltaSeconds :type "Float (single-precision)"))
  (bind _returnvalue (- (`self.K2_GetActorLocation` (`GameplayStatics.GetPlayerPawn` 0)) (`self.K2_GetActorLocation`)))
  ;[1 1 1] Rotate Turret towards character
  (bind _output_get (set `self.Triggered` (<= (`KismetMathLibrary.VSize` _returnvalue) (`self.TriggerDistance`))))
  (if _output_get
    (`SceneComponent.K2_SetWorldRotation` (`self.Cylinder`) (`KismetMathLibrary.MakeRotator` 0.0 0.0 (.yaw (`KismetMathLibrary.MakeRotationFromAxes` _returnvalue))) false false)))

(event `self.ReceiveBeginPlay`
  ;[1 1 1] Shooting
  (`KismetSystemLibrary.K2_SetTimerDelegate` (delegate `Shoot`) 1.0 true))

(event `Shoot`
  (bind _shootingdirection (`self.ShootingDirection`))
  (bind _returnvalue (`SceneComponent.K2_GetComponentLocation` _shootingdirection))
  ;[1 1 1] Shooting
  (if (`self.Triggered`)
    (bind _outhit (`KismetSystemLibrary.LineTraceSingle` :`Start` _returnvalue :`End` (+ _returnvalue (* (`KismetMathLibrary.GetForwardVector` (`SceneComponent.K2_GetComponentRotation` _shootingdirection)) 3000)) :`TraceChannel` "TraceTypeQuery2" :`bTraceComplex` true :`DrawDebugType` "ForDuration"))
    (`self.Charge`)
    (message `/Game/ThirdPerson/Blueprints/BPI_Shooting.ApplyDamage` (`.HitActor` (`GameplayStatics.BreakHitResult` _outhit)) 10.0)
    (`ActorComponent.SetActive` (`self.MuzzleFlash`) true true)))

(event `Charge`
  ;[1 1 1] Carica
  (bind (_direction _newtrack_0) (`Timeline|Timeline` :!via `PlayFromStart`)
    (:`Update`
      (`SceneComponent.K2_SetRelativeLocation` (`self.Cannon`) (`KismetMathLibrary.MakeVector` (`KismetMathLibrary.Lerp` 53.0 63.0 _newtrack_0)) false false))))

(fn `UserConstructionScript`)
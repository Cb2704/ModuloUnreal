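; BP_Door is a door actor that rises once enough triggers have reported in.
; Each UpdateCounter call increments TriggerCounter and calls MoveDoor when it equals MaxTrigger.
; MoveDoor plays a timeline that adds a lerped Z step to the door's current position every update, so movement accumulates per frame.
; Tick separately prunes invalid entries from TriggerReferences, which does not affect the counter.
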(event `self.ReceiveTick`
  (params (DeltaSeconds :type "Float (single-precision)"))
  (for (_array_element _array_index) (`self.Trigger References`)
    (if (not (`KismetSystemLibrary.IsValid` _array_element))
      (`KismetArrayLibrary.Array_Remove` (`self.Trigger References`) _array_index))))

(event `UpdateCounter`
  (`/Engine/EditorBlueprintResources/StandardMacros.IncrementInt` (`self.TriggerCounter`)
    (:`  `
      (if (== (`self.TriggerCounter`) (`self.MaxTrigger`))
        (`self.MoveDoor`)))))

(event `MoveDoor`
  (bind (_returnvalue_x _returnvalue_y _returnvalue_z) (`KismetMathLibrary.BreakVector` (`SceneComponent.K2_GetComponentLocation` (`self.Door`))))
  (bind (_direction _valore_uscita) (`Timeline|Timeline`)
    (:`Update`
      (`SceneComponent.K2_SetWorldLocation` (`self.Door`) (`KismetMathLibrary.MakeVector` _returnvalue_x _returnvalue_y (+ _returnvalue_z (`KismetMathLibrary.Lerp` 0.0 3.0 _valore_uscita))) false false))))

(fn `UserConstructionScript`)